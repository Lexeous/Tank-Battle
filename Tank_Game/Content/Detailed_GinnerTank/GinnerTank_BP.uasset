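; Player-controlled tank Blueprint that binds input to driving, camera-gimbal aiming and firing.
; On BeginPlay it hands the barrel and turret to the TankAiming component and both tracks to TankMovement.
; Move and turn axes feed TankMovement intents, and the FIRE action calls TankAiming.Fire.
; Aim axes rotate separate azimuth (yaw) and elevation (pitch) gimbal components locally, scaled by delta time for frame-rate independence.
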(event `self.ReceiveBeginPlay`
  (`TankAimingComponent.Initialise` (`self.TankAiming`) (`self.Ginner_Barrel`) (`self.Ginner_Turret`))
  (`TankMovementComponent.Initialise` (`self.TankMovement`) (`self.Left_Track`) (`self.Right_Track`)))

(event `InputAxis|AimAzimuth`
  (params (AxisValue :type "Float (single-precision)"))
  ;[1 1 1] Ballisticts Input Binding
  (`SceneComponent.K2_AddLocalRotation` (`self.AzimuthGimble`) (`KismetMathLibrary.MakeRotator` 0.0 0.0 (* AxisValue (`GameplayStatics.GetWorldDeltaSeconds`) 100.0)) false false))

(event `InputAxis|Move Forward`
  (params (AxisValue :type "Float (single-precision)"))
  ;[1 1 1] Movement input binding
  (`TankMovementComponent.IntendMoveForward` (`self.TankMovement`) AxisValue))

(event `InputAxis|Turn Right`
  (params (AxisValue :type "Float (single-precision)"))
  ;[1 1 1] Movement input binding
  (`TankMovementComponent.IntendTurnRight` (`self.TankMovement`) AxisValue))

(event `InputAxis|AimElevation`
  (params (AxisValue :type "Float (single-precision)"))
  ;[1 1 1] Ballisticts Input Binding
  (`SceneComponent.K2_AddLocalRotation` (`self.Elevation`) (`KismetMathLibrary.MakeRotator` 0.0 (* AxisValue (`GameplayStatics.GetWorldDeltaSeconds`) 100.0)) false false))

(event `InputAction|FIRE`
  (params (Key :type "Key Structure" :default "AnyKey"))
  ;[1 1 1] Ballisticts Input Binding
  (:`Pressed`
    (`TankAimingComponent.Fire` (`self.TankAiming`))))

(fn `UserConstructionScript`)